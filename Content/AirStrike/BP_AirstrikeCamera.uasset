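; BP_AirstrikeCamera is a possessable pawn that lets the player call in airstrikes through a UI.
; SwitchToCamera stores the player's current pawn and possesses the camera, which opens W_Airstrike with UI-only input and a visible cursor.
; On completion, OnAirstrikeComplete spawns a BP_AirstrikeExplosion at each supplied location and repossesses the stored pawn.
; Unpossession removes the widget, but input mode and cursor are not restored here.
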(event `Switch To Camera`
  (params (`Player Controller` :type "PlayerController Object Reference"))
  (set `self.Controlling Pawn` (`Controller.K2_GetPawn` `Player Controller`))
  (`Controller.Possess` `Player Controller` self))

(event `self.ReceivePossessed`
  (params (NewController :type "Controller Object Reference"))
  (bind _airstrike_widget (`self.Airstrike Widget`))
  (bind _asplayer_controller (cast `PlayerController` NewController))
  (bind _returnvalue (`|CreateWidget` "/Game/AirStrike/W_Airstrike.W_Airstrike_C" _asplayer_controller))
  (bind _output_get (set `self.Airstrike Widget` _returnvalue))
  (add `/Game/AirStrike/W_Airstrike.On Complete` _output_get (`|CreateDelegate` :!event `On Airstrike Complete`))
  (`UserWidget.AddToViewport` _airstrike_widget 0)
  (`WidgetBlueprintLibrary.SetInputMode_UIOnlyEx` _asplayer_controller _airstrike_widget "LockAlways")
  (set `PlayerController.bShowMouseCursor` true _asplayer_controller))

(event `self.ReceiveUnpossessed`
  (params (OldController :type "Controller Object Reference"))
  (cast `PlayerController` OldController)
  (bind _airstrike_widget (`self.Airstrike Widget`)
    (:`then`
      (if (`Widget.IsInViewport` _airstrike_widget)
        (`Widget.RemoveFromParent` (`self.Airstrike Widget`))
        (set `self.Airstrike Widget` null)))
    (:`else`)))

(fn `On Airstrike Complete`
  (params (`Airstrike Locations` :type "Array of Vector Structure (by ref)"))
  (for _array_element `Airstrike Locations`
    (`|SpawnActorFromClass` "/Game/AirStrike/BP_AirstrikeExplosion.BP_AirstrikeExplosion_C" (`KismetMathLibrary.MakeTransform` _array_element) "Undefined" "MultiplyWithRoot" null null))
  (`Controller.Possess` (`self.GetController`) (`self.Controlling Pawn`))
  (return))

(fn `UserConstructionScript`)