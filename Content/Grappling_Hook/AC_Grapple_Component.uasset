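; Actor component that gives a Character a grappling hook, firing a hook projectile and pulling the owner toward whatever it hits.
; FireGrapple spawns the hook and a cable actor linked to it, binding hit and destroyed events.
; A hit removes friction and gravity and launches the owner, and Tick keeps adding pulling force.
; The hook is destroyed when close or overshot (2D dot-product check), resetting movement and state.
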(event `self.ReceiveTick`
  (params (DeltaSeconds :type "Float (single-precision)"))
  (switch `/Game/Grappling_Hook/E_GrappleState` (`self.Grapple State`)
    (:`NewEnumerator2`
      (bind _ascharacter (cast `Character` (`self.GetOwner`)))
      (`CharacterMovementComponent.AddForce` (`Character.CharacterMovement` _ascharacter) (* (`self.To Grapple Hook`) 100000.0))
      (if (< (`KismetMathLibrary.Vector_Distance` (`Actor.K2_GetActorLocation` (`self.Grapple Hook`)) (`Actor.K2_GetActorLocation` (`self.GetOwner`))) 250.0)
        (`Actor.K2_DestroyActor` (`self.Grapple Hook`))
        (elif (< (`KismetMathLibrary.Dot_VectorVector` (`self.Inital Hook 2D`) (`self.To Grapple Hook 2D`)) 0.0)
          (`Actor.K2_DestroyActor` (`self.Grapple Hook`)))))))

(fn `Cancel Grapple`
  (bind _grapple_hook (`self.Grapple Hook`)
    (:`then`
      (`Actor.K2_DestroyActor` _grapple_hook))
    (:`else`)))

(fn `Fire Grapple`
  (params (`Target Location` :type "Vector Structure") (`Local Offest` :type "Vector Structure"))
  (locals (`Fire Direction` :type "Vector Structure" :default (0.0 0.0 0.0)))
  (if (not (`self.Is in Use?`))
    (set `self.Grapple State` "NewEnumerator1")
    (set `local.Fire Direction` (`KismetMathLibrary.Normal` (- (`local.Target Location`) (`self.Cable Start Location` (`local.Local Offest`)))))
    (bind _returnvalue (`|SpawnActorFromClass` "/Game/Grappling_Hook/BP_GrappleHook.BP_GrappleHook_C" (`KismetMathLibrary.MakeTransform` (`self.Cable Start Location` (`local.Local Offest`))) "Undefined" "MultiplyWithRoot" null (* (`local.Fire Direction`) (`self.Speed`)) 3500.0 null))
    (bind _output_get (set `self.Grapple Hook` _returnvalue))
    (add `Actor.OnActorHit` _output_get (`|CreateDelegate` :!event `On Grapple Hit`))
    (add `Actor.OnDestroyed` (`self.Grapple Hook`) (`|CreateDelegate` :!event `On Grapple Hook Destroyed`))
    (bind _returnvalue_2 (`|SpawnActorFromClass` "/Game/Grappling_Hook/BP_CA_GrappleCable.BP_CA_GrappleCable_C" (`KismetMathLibrary.MakeTransform` (`self.Cable Start Location` (`local.Local Offest`)) (`KismetMathLibrary.MakeRotFromX` (`local.Fire Direction`))) "Undefined" "MultiplyWithRoot" null null))
    (bind _output_get_2 (set `self.Grapple Cable` _returnvalue_2))
    (`Actor.K2_AttachToActor` _output_get_2 (`self.GetOwner`) "None" "KeepWorld" "KeepWorld" "KeepWorld" true)
    (`CableComponent.SetAttachEndTo` (`CableActor.CableComponent` (`self.Grapple Cable`)) (`self.Grapple Hook`) "None" "None")
    (set `CableComponent.EndLocation` (0.0 0.0 0.0) (`CableActor.CableComponent` (`self.Grapple Cable`))) ; Keep 0:0:0
  ))

(fn `Is in Use?`
  (returns (Result :type Boolean))
  (return (select `/Game/Grappling_Hook/E_GrappleState` (`self.Grapple State`) :`NewEnumerator1` true :`NewEnumerator2` true)))

(fn `On Grapple Hit`
  (params (SelfActor :type "Actor Object Reference") (OtherActor :type "Actor Object Reference") (NormalImpulse :type "Vector Structure") (Hit :type "HitResult Structure (by ref)"))
  (set `self.Grapple State` "NewEnumerator2")
  (bind _ascharacter (cast `Character` (`self.GetOwner`)))
  (bind _charactermovement (`Character.CharacterMovement` _ascharacter))
  (set `CharacterMovementComponent.GroundFriction` 0.0 _charactermovement)
  (set `CharacterMovementComponent.GravityScale` 0.0 _charactermovement)
  (set `CharacterMovementComponent.AirControl` 0.2 _charactermovement)
  (set `MovementComponent.Velocity` (* (`self.To Grapple Hook`) 1200.0) _charactermovement)
  (set `self.Inital Hook 2D` (`self.To Grapple Hook 2D`)))

(fn `On Grapple Hook Destroyed`
  (params (DestroyedActor :type "Actor Object Reference"))
  (set `self.Grapple Hook` null)
  (set `self.Grapple State` "NewEnumerator0")
  (`|ExecutionSequence`
    (:`then_0`
      (bind _grapple_cable (`self.Grapple Cable`)
        (:`then`
          (`Actor.K2_DestroyActor` _grapple_cable)
          (set `self.Grapple Cable` null))
        (:`else`)))
    (:`then_1`
      (bind _ascharacter (cast `Character` (`self.GetOwner`)))
      (bind _charactermovement (`Character.CharacterMovement` _ascharacter))
      (set `CharacterMovementComponent.GroundFriction` 1.0 _charactermovement)
      (set `CharacterMovementComponent.GravityScale` 1.0 _charactermovement)
      (set `CharacterMovementComponent.AirControl` 0.05 _charactermovement))))