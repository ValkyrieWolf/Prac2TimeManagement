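; BP_OBJ_Item is an inventory item object holding its grid dimensions, icons, item class and rotation state.
; Rotate toggles the Rotated flag, and GetDimensions swaps X and Y while it is set.
; GetIcon returns a separate rotated icon in that state, and simple getters expose the item class and rotation flag.
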(fn `Get Dimensions`
  (returns (Dimensions :type "IntPoint Structure"))
  (bind (_dimensions_x _dimensions_y) (break `IntPoint` (`self.Dimensions`)))
  (if (`self.Rotated`)
    (return (make `IntPoint` _dimensions_y _dimensions_x))
    (else
      (return (`self.Dimensions`)))))

(fn `Get Icon`
  (returns (Icon :type "MaterialInterface Object Reference"))
  (return (select `bool` (`self.Rotated`) :`false` (`self.Icon`) :`true` (`self.Icon Rotated`))))

(fn `Get Item Class`
  (returns (`Item Class` :type "/Game/Inventory_System/Items/Parent/BP_Item Class Reference"))
  (return (`self.Item Class`)))

(fn `Is Rotated`
  (returns (Rotated :type Boolean))
  (return (`self.Rotated`)))

(fn `Rotate`
  (set `self.Rotated` (not (`self.Rotated`))))