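; BP_Item is the parent Blueprint for world item pickups that go into the player's inventory.
; On BeginPlay, it fills an invalid ItemObject from GetDefaultItemObject, which returns nothing here and appears intended for child overrides.
; When a BP_ThirdPersonCharacter overlaps the Sphere, it passes ItemObject to that character's ACInventory through TryAddItem.
; The actor destroys itself only if the add succeeds.
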(event `self.ReceiveBeginPlay`
  (if (not (`KismetSystemLibrary.IsValid` (`self.Item Object`)))
    (bind _item_object (`self.Get Default Item Object`))
    (set `self.Item Object` _item_object)))

(event `self.Sphere.OnComponentBeginOverlap`
  (params (OverlappedComponent :type "PrimitiveComponent Object Reference") (OtherActor :type "Actor Object Reference") (OtherComp :type "PrimitiveComponent Object Reference") (OtherBodyIndex :type Integer) (bFromSweep :type Boolean) (SweepResult :type "HitResult Structure (by ref)"))
  (bind _asbp_third_person_character (cast `/Game/ThirdPerson/Blueprints/BP_ThirdPersonCharacter` OtherActor))
  (bind _added (`/Game/Inventory_System/AC_Inventory.Try Add Item` (`/Game/ThirdPerson/Blueprints/BP_ThirdPersonCharacter.AC_Inventory` _asbp_third_person_character) (`self.Item Object`)))
  (if _added
    (`self.K2_DestroyActor`)))

(fn `Get Default Item Object`
  (returns (`Item Object` :type "/Game/Items/BP_OBJ_Item Object Reference"))
  (return null))

(fn `UserConstructionScript`)