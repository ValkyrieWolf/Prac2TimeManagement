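; Portal component that places portal A or B on portal walls by tracing from a given start location and direction.
; SpawnPortalAlongVector runs a debug-drawn line trace on a single object type, with its end computed as start plus direction, both scaled by MaxSpawnDistance.
; A BP_PortalWall hit receives TryAddPortal with the impact location nudged slightly back along the trace and the PortalA flag.
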(fn `Spawn Portal Along Vector`
  (params (`Start Location` :type "Vector Structure") (Direction :type "Vector Structure") (`Portal A` :type Boolean))
  (bind (_outhit _returnvalue) (`KismetSystemLibrary.LineTraceSingleForObjects` :`Start` (`local.Start Location`) :`End` (* (+ (`local.Start Location`) (`local.Direction`)) (`self.Max Spawn Distance`)) :`ObjectTypes` (`|MakeArray` "ObjectTypeQuery7" :!type "EObjectTypeQuery Enum") :`DrawDebugType` "ForDuration" :`DrawTime` 1.5))
  (if _returnvalue
    (bind (_bblockinghit _binitialoverlap _time _distance _location _impactpoint _normal _impactnormal _physmat _hitactor _hitcomponent _hitbonename _bonename _hititem _elementindex _faceindex _tracestart _traceend) (`GameplayStatics.BreakHitResult` _outhit))
    (bind _asbp_portal_wall (cast `/Game/Portal/BP_PortalWall` _hitactor))
    (`/Game/Portal/BP_PortalWall.Try Add Portal` _asbp_portal_wall (+ _location (* (`KismetMathLibrary.Normal` (- _tracestart _traceend)) 1.0)) (`local.Portal A`))))