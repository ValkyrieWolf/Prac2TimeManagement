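; BP_PortalWall is a wall actor that accepts portal placement, with its mesh scaled from width and height in the construction script.
; TryAddPortal converts the requested origin to wall-local space, nudges it inward so the portal fits within the edges, then rejects rectangle overlaps with existing portals.
; Valid placements spawn a BP_Portal aligned to the wall and track it in PortalsOnWall until its destroyed event removes it.
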(fn `Clamp Point To Wall`
  (params (Point :type "Float (double-precision)") (`Wall Size` :type "Float (double-precision)") (`Portal Radius` :type "Float (double-precision)"))
  (returns (ReturnValue :type "Float (double-precision)"))
  (locals (`Offset (Local)` :type "Float (double-precision)" :default 0.0))
  ;[0.8443 0 1] Math that takes a point along x or y that will figure out, how much we need to move the point inwards to see how much it needs to stay inside the wall.
  (bind _output_get (set `local.Offset (Local)` (`KismetMathLibrary.FClamp` (- (- (/ `Wall Size` 2.0) (`local.Portal Radius`)) (`KismetMathLibrary.Abs` (`local.Point`))) -1e+53 0.0)))
  (set `local.Offset (Local)` (* (`local.Offset (Local)`) (select `bool` (< (`local.Point`) 0.0) :`false` -1.0 :`true` 1.0)))
  (return (- (`local.Point`) _output_get)))

(fn `Constrain Portal To Wall`
  (params (`Portal Y` :type "Float (double-precision)") (`Portal Z` :type "Float (double-precision)"))
  (returns (`Constrained Y` :type "Float (double-precision)") (`Constrained Z` :type "Float (double-precision)"))
  (locals (`Clamped Y (Local)` :type "Float (double-precision)" :default 0.0) (`Clamped Z (Local)` :type "Float (double-precision)" :default 0.0))
  ;[0 0.2691 1] Clamped Y Value
  (bind _returnvalue (`self.Clamp Point To Wall` (`local.Portal Y`) (`self.Wall Width`) (`self.Portal Size`)))
  (set `local.Clamped Y (Local)` _returnvalue)
  ;[0 0.1435 1] Clamped Z
  (bind _returnvalue_2 (`self.Clamp Point To Wall` (`local.Portal Z`) (`self.Wall Height`) (`.Radius Z` (`self.Portal Size`))))
  (set `local.Clamped Z (Local)` _returnvalue_2)
  (return (`local.Clamped Y (Local)`) (`local.Clamped Z (Local)`)))

(fn `Has Room For New Portal?`
  (params (`New Portal Y` :type "Float (double-precision)") (`New Portal Z` :type "Float (double-precision)"))
  (returns (Result :type Boolean))
  (bind (_radius_y _radius_z) (`self.Portal Size`))
  (bind _returnvalue (`KismetMathLibrary.MakeVector2D` _radius_y _radius_z))
  (for _array_element (`self.Portals On Wall`)
    (bind (_returnvalue_x _returnvalue_y _returnvalue_z) (`KismetMathLibrary.BreakVector` (`KismetMathLibrary.InverseTransformLocation` (`self.GetTransform`) (`self.K2_GetActorLocation` _array_element))))
    (if (`/Game/Function_Library/BPF_MyFunctionLibrary.Rectangle to Rectangle Collision` (`KismetMathLibrary.MakeVector2D` _returnvalue_y _returnvalue_z) _returnvalue (`KismetMathLibrary.MakeVector2D` (`local.New Portal Y`) (`local.New Portal Z`)) _returnvalue)
      (return false)))
  (return true))

(fn `On Portal Destroyed`
  (params (DestroyedActor :type "Actor Object Reference"))
  (`KismetArrayLibrary.Array_RemoveItem` (`self.Portals On Wall`) DestroyedActor))

(fn `Try Add Portal`
  (params (`Portal Origin` :type "Vector Structure") (`Portal A` :type Boolean))
  (returns (`New Portal` :type "/Game/Portal/BP_Portal Object Reference"))
  (locals (`Relative Portal Origin (Local)` :type "Vector Structure" :default (0.0 0.0 0.0)))
  (bind (_relative_portal_origin__local__x _relative_portal_origin__local__y _relative_portal_origin__local__z) (`KismetMathLibrary.BreakVector` (`local.Relative Portal Origin (Local)`)))
  (bind _relative_portal_origin__local__x_2 (`KismetMathLibrary.BreakVector` (`local.Relative Portal Origin (Local)`)))
  (bind (_relative_portal_origin__local__x_3 _relative_portal_origin__local__y_2 _relative_portal_origin__local__z_2) (`KismetMathLibrary.BreakVector` (`local.Relative Portal Origin (Local)`)))
  (set `local.Relative Portal Origin (Local)` (`KismetMathLibrary.InverseTransformLocation` (`self.GetTransform`) (`local.Portal Origin`)))
  (bind (_constrained_y _constrained_z) (`self.Constrain Portal To Wall` _relative_portal_origin__local__y _relative_portal_origin__local__z))
  (set `local.Relative Portal Origin (Local)` (`KismetMathLibrary.MakeVector` _relative_portal_origin__local__x_2 _constrained_y _constrained_z))
  (if (`self.Has Room For New Portal?` _relative_portal_origin__local__y_2 _relative_portal_origin__local__z_2)
    (bind _returnvalue (`|SpawnActorFromClass` "/Game/Portal/BP_Portal.BP_Portal_C" (`KismetMathLibrary.MakeTransform` (`KismetMathLibrary.TransformLocation` (`self.GetTransform`) (`local.Relative Portal Origin (Local)`)) (`self.K2_GetActorRotation`)) "AlwaysSpawn" "MultiplyWithRoot" null (`local.Portal A`) null))
    (`KismetArrayLibrary.Array_Add` (`self.Portals On Wall`) _returnvalue)
    (add `self.OnDestroyed` _returnvalue (`|CreateDelegate` :!event `On Portal Destroyed`))
    (return _returnvalue)))

(fn `UserConstructionScript`
  (`SceneComponent.SetWorldScale3D` (`self.StaticMesh`) (`KismetMathLibrary.MakeVector` 1.0 (/ (`self.Wall Width`) 100.0) (/ (`self.Wall Height`) 100.0))))