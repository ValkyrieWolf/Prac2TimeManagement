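; Vaulting component for BP_ThirdPersonCharacter that detects climbable ledges ahead and moves the character onto them.
; While idle, Tick runs a vertical line trace ahead, validates ledge height, walkable slope and capsule clearance, then toggles a W_Vault widget.
; Vault switches state, and Tick then lerps the actor to the cached ledge location without sweeping, using VaultSpeed as duration.
; Trace and capsule debug drawing are enabled.
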(event `self.ReceiveBeginPlay`
  (bind _asbp_third_person_character (cast `/Game/ThirdPerson/Blueprints/BP_ThirdPersonCharacter` (`self.GetOwner`)))
  (set `self.Owning Character` _asbp_third_person_character)
  (bind _returnvalue (`|CreateWidget` "/Game/Vaulting/W_Vault.W_Vault_C" (cast `PlayerController` (`Pawn.GetController` (`self.Owning Character`)) :!pure true)))
  (set `self.Vault Widget` _returnvalue))

(event `self.ReceiveTick`
  (params (DeltaSeconds :type "Float (single-precision)"))
  (`self.Switch Vaulting State`
    (:`Not Vaulting`
      (bind (_result _ending_location) (`self.Can Vault`))
      (if _result
        (set `self.Ending Location` _ending_location)
        (if (not (`Widget.IsInViewport` (`self.Vault Widget`)))
          (`UserWidget.AddToViewport` (`self.Vault Widget`) 0))
        (elif (`Widget.IsInViewport` (`self.Vault Widget`))
          (`Widget.RemoveFromParent` (`self.Vault Widget`)))))
    (:`Vaulting`
      (`self.Tick Vault` DeltaSeconds))))

(event `Vault`
  (set `self.Progress` 0.0)
  (set `self.Starting Location` (`Actor.K2_GetActorLocation` (`self.Owning Character`)))
  (set `self.Vaulting State` "NewEnumerator2"))

(fn `Can Vault`
  (returns (Result :type Boolean) (`Ending Location` :type "Vector Structure"))
  (locals (`Capsule (Local)` :type "CapsuleComponent Object Reference"))
  (bind _owning_character (`self.Owning Character`))
  (bind _returnvalue (`CapsuleComponent.GetScaledCapsuleHalfHeight` (`Character.CapsuleComponent` (`self.Owning Character`))))
  (bind _returnvalue_2 (+ (`Actor.K2_GetActorLocation` _owning_character) (* (`Actor.GetActorForwardVector` _owning_character) 70.0)))
  (if (`|EnumEquality` (`self.Vaulting State`) "NewEnumerator0")
    (set `local.Capsule (Local)` (`Character.CapsuleComponent` (`self.Owning Character`)))
    (bind (_outhit _returnvalue_3) (`KismetSystemLibrary.LineTraceSingle` (+ _returnvalue_2 (`KismetMathLibrary.MakeVector` 0.0 0.0 _returnvalue)) (- _returnvalue_2 (`KismetMathLibrary.MakeVector` 0.0 0.0 _returnvalue)) "TraceTypeQuery1" false (`|MakeArray` (`self.Owning Character`) :!type "Actor Object Reference") "ForOneFrame"))
    (if _returnvalue_3
      (bind (_result _ending_location) (`self.Can Vault to Hit` (`local.Capsule (Local)`) _outhit))
      (return _result _ending_location)
      (else
        (return false (0.0 0.0 0.0))))
    (else
      (return false (0.0 0.0 0.0)))))

(fn `Can Vault to Hit`
  (params (Capsule :type "CapsuleComponent Object Reference") (Hit :type "HitResult Structure"))
  (returns (Result :type Boolean) (`Ending Location` :type "Vector Structure"))
  (locals (`Ending Location (Local)` :type "Vector Structure" :default (0.0 0.0 0.0)))
  (bind (_hit_bblockinghit _hit_binitialoverlap _hit_time _hit_distance _hit_location) (`GameplayStatics.BreakHitResult` (`local.Hit`)))
  (bind (_hit_bblockinghit_2 _hit_binitialoverlap_2 _hit_time_2 _hit_distance_2 _hit_location_2 _hit_impactpoint _hit_normal _hit_impactnormal _hit_physmat _hit_hitactor _hit_hitcomponent _hit_hitbonename _hit_bonename _hit_hititem _hit_elementindex _hit_faceindex _hit_tracestart _hit_traceend) (`GameplayStatics.BreakHitResult` (`local.Hit`)))
  (bind (_hit_bblockinghit_3 _hit_binitialoverlap_3 _hit_time_3 _hit_distance_3 _hit_location_3 _hit_impactpoint_2 _hit_normal_2) (`GameplayStatics.BreakHitResult` (`local.Hit`)))
  (bind _capsule (`local.Capsule`))
  (bind _returnvalue (`CapsuleComponent.GetScaledCapsuleRadius` _capsule))
  (`|ExecutionSequence`
    (:`then_0`
      ;[0.2247 1 0.7882] Making sure that the ledge is at an approriate height!
      (if (not (`KismetMathLibrary.InRange_FloatFloat` (- (.z _hit_location_2) (.z _hit_traceend)) (`self.Min Vaulting Height`) (`self.Max Vaulting Height`)))
        (return false (0.0 0.0 0.0))))
    (:`then_1`
      ;[0.3022 1 0.8372] Make sure the Surface we are vaulting to is walkable!
      (if (< (.z _hit_normal_2) (`CharacterMovementComponent.K2_GetWalkableFloorZ` (`Character.CharacterMovement` (`self.Owning Character`))))
        (return false (0.0 0.0 0.0))))
    (:`then_2`
      ;[1 1 1] Make sure there is enough room for us on top of the ledge
      (bind _output_get (set `local.Ending Location (Local)` (+ _hit_location (`KismetMathLibrary.MakeVector` 0.0 0.0 (`CapsuleComponent.GetScaledCapsuleHalfHeight` (`local.Capsule`))))))
      (bind _result (`self.Check Capsule Collision` (+ _output_get (`KismetMathLibrary.MakeVector` 0.0 0.0 _returnvalue)) (`CapsuleComponent.GetScaledCapsuleHalfHeight` _capsule) _returnvalue true))
      (if _result
        (return false (0.0 0.0 0.0))))
    (:`then_3`
      (return true (`local.Ending Location (Local)`)))))

(fn `Check Capsule Collision`
  (params (Center :type "Vector Structure") (`Half Height` :type "Float (double-precision)") (Radius :type "Float (double-precision)") (`Draw Debug` :type Boolean))
  (returns (Result :type Boolean))
  (`|ExecutionSequence`
    (:`then_0`
      (if (`local.Draw Debug`)
        (`KismetSystemLibrary.DrawDebugCapsule` (`local.Center`) (`local.Half Height`) (`local.Radius`) (struct) (struct :`R` 0.653641 :`G` 0.664583 :`A` 1.0) 0.0 3.0)))
    (:`then_1`
      (bind (_outactors _returnvalue) (`KismetSystemLibrary.CapsuleOverlapActors` (`local.Center`) (`local.Radius`) (`local.Half Height`) (`|MakeArray` "ObjectTypeQuery1" "ObjectTypeQuery2" "ObjectTypeQuery4" "ObjectTypeQuery5" "ObjectTypeQuery6" :!type "EObjectTypeQuery Enum") "/Script/Engine.Actor" (`|MakeArray` (`self.Owning Character`) :!type "Actor Object Reference")))
      (return _returnvalue))))

(fn `Tick Vault`
  (params (`Delta Seconds` :type "Float (double-precision)"))
  (`|ExecutionSequence`
    (:`then_0`
      (set `self.Progress` (`KismetMathLibrary.FClamp` (+ (`self.Progress`) (/ (`local.Delta Seconds`) (`self.Vault Speed`)))))
      (`Actor.K2_SetActorLocation` (`self.Owning Character`) (`KismetMathLibrary.VLerp` (`self.Starting Location`) (`self.Ending Location`) (`self.Progress`)) false true))
    (:`then_1`
      (if (>= (`self.Progress`) 1.0)
        (set `self.Vaulting State` "NewEnumerator0")))))